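; BP_PlayerKart is the player's kart Blueprint, handling its engine audio, horn and propeller animation.
; Each tick, SpeedRatio drives the engine sound's RPM parameter and spins the Helice propeller at a frame-rate-independent rate.
; The klaxon input plays the horn, while BeginPlay silences the horn and drift audio.
; SpeedRatio is only read in this graph, and drift audio is never started here.
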(event EventBeginPlay
  (Audio|Components|Audio|Stop (Variables|Default|Getklaxon))
  (Audio|Components|Audio|Stop (Variables|Default|GetdriftAudioComp)))

(event Collision|EventActorBeginOverlap
  (params (OtherActor :type Actor%20Object%20Reference)))

(event EventTick
  (params (DeltaSeconds :type Float%20%28single-precision%29))
  (Audio|Parameter|SetFloatParameter (Variables|Default|GetEngineSoundComp) "RPM" (Variables|Default|GetspeedRatio) :!class /Script/AudioExtensions.AudioParameterControllerInterface)
  (Transformation|AddLocalRotation (Variables|Default|Gethelice) (Math|Rotator|MakeRotator 0.0 (* (Variables|Default|GetspeedRatio) DeltaSeconds 8e+02) 0.0) false false))

(event Input|ActionEvents|InputActionklaxon
  (params (Key :type Key%20Structure :default "None"))
  (:Pressed
    (Audio|Components|Audio|Play (Variables|Default|Getklaxon) 0.0)))

(fn ConstructionScript)